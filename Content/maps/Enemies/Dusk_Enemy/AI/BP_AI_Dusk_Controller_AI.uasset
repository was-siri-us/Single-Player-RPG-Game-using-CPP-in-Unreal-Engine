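; BP_AI_Dusk_Controller_AI is the AI controller for the Dusk enemy, handling detection and chase targeting.
; It runs the BT_Dusk_AI behavior tree on BeginPlay.
; AI perception updates feed the TargetActor blackboard key, storing any actor successfully sensed by sight, without filtering.
; A lost sight stimulus, or any update from another sense, clears that key.
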(event `self.ReceiveBeginPlay`
  (`self.RunBehaviorTree` "/Game/maps/Enemies/Dusk_Enemy/AI/BT_Dusk_AI.BT_Dusk_AI"))

(event `self.AIPerception.OnTargetPerceptionUpdated`
  (params (Actor :type "Actor Object Reference") (Stimulus :type "AIStimulus Structure"))
  ;[0.003737 0.3926 1] Detect and Chase
  (bind _returnvalue (`AIPerceptionSystem.GetSenseClassForStimulus` Stimulus))
  (if (== _returnvalue "/Script/AIModule.AISense_Sight")
    (if (`.bSuccessfullySensed` (break `AIStimulus` Stimulus))
      (`BlackboardComponent.SetValueAsObject` (`AIBlueprintHelperLibrary.GetBlackboard` self) "TargetActor" Actor)
      (else
        (`BlackboardComponent.SetValueAsObject` (`AIBlueprintHelperLibrary.GetBlackboard` self) "TargetActor" null :!label _label)))
    (else
      (goto _label))))

(fn `UserConstructionScript`)