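; Dusk enemy minion that performs a four-step melee combo against the Aurora player character.
; The Attack function triggers the combo if CanAttack is set, buffers repeat requests in SaveAttack and returns a fixed duration.
; MinionComboAttack either continues to the AttackIndex step or resets the combo.
; Each step plays its montage, then sphere-checks at EnemyPosArrow to apply damage, sound and sparks.
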(event `self.ReceiveBeginPlay`
  (`SceneComponent.K2_AttachToComponent` (`self.Sphere`) null "foot_l" "KeepRelative" "KeepRelative" "KeepRelative" true)
  (`SceneComponent.K2_AttachToComponent` (`self.Sphere1`) null "foot_r" "KeepRelative" "KeepRelative" "KeepRelative" true))

(event `MinionAttack1`
  (bind _enemyposarrow (`self.EnemyPosArrow`))
  (bind _returnvalue (`SceneComponent.K2_GetComponentLocation` _enemyposarrow))
  (`/Engine/EditorBlueprintResources/StandardMacros.DoOnce` false :!label _label
    (:`Completed`
      (`KismetSystemLibrary.Delay` 0.1)
      (`self.PlayAnimMontage` "/Game/maps/Enemies/PrimeHelix/Animations/attacka.attacka")
      (bind _outactors (`KismetSystemLibrary.SphereOverlapActors` (`SceneComponent.K2_GetComponentLocation` (`self.EnemyPosArrow`)) 50.0 (`|MakeArray` "ObjectTypeQuery3" :!type "EObjectTypeQuery Enum") "/Game/maps/PlayerAssets/MyAuroraCharacter_BP.MyAuroraCharacter_BP_C" (`|MakeArray` self :!type "Actor Object Reference")))
      (for _array_element _outactors
        (`GameplayStatics.ApplyDamage` _array_element 2.5)
        (`GameplayStatics.PlaySoundAtLocation` null _returnvalue (struct) 1.0 1.0 0.0 null null null)
        (`GameplayStatics.SpawnEmitterAtLocation` "/Game/InfinityBladeEffects/Effects/FX_Monsters/FX_Monster_Ausar/P_AU_Taunt_sparks.P_AU_Taunt_sparks" _returnvalue (`SceneComponent.K2_GetComponentRotation` _enemyposarrow)))
      (set `self.AttackIndex` 1)
      (goto _label :!via `Reset`))))

(event `MinionComboAttackBTcall`
  (if (`self.canAttack`)
    (`self.MinionAttack`)))

(event `MinionAttack`
  (if (`self.isAttacking`)
    (set `self.SaveAttack` true)
    (else
      (set `self.isAttacking` true)
      (switch `int` (`self.AttackIndex`) :!label _label_2
        (:`0`
          (`self.MinionAttack1`))
        (:`1`
          (`self.MinionAttack2`))
        (:`2`
          (`self.MinionAttack3`))
        (:`3`
          (`self.MinionAttack4`))))))

(event `MinionComboAttack`
  (if (`self.SaveAttack`)
    (set `self.SaveAttack` false)
    (goto _label_2)
    (else
      (`self.StopMinionCombo`))))

(event `MinionAttack2`
  (bind _enemyposarrow (`self.EnemyPosArrow`))
  (bind _returnvalue (`SceneComponent.K2_GetComponentLocation` _enemyposarrow))
  (`/Engine/EditorBlueprintResources/StandardMacros.DoOnce` false :!label _label_3
    (:`Completed`
      (`KismetSystemLibrary.Delay` 0.1)
      (`self.PlayAnimMontage` "/Game/maps/Enemies/PrimeHelix/Animations/attackB.attackB")
      (bind _outactors (`KismetSystemLibrary.SphereOverlapActors` (`SceneComponent.K2_GetComponentLocation` (`self.EnemyPosArrow`)) 50.0 (`|MakeArray` "ObjectTypeQuery3" :!type "EObjectTypeQuery Enum") "/Game/maps/PlayerAssets/MyAuroraCharacter_BP.MyAuroraCharacter_BP_C" (`|MakeArray` self :!type "Actor Object Reference")))
      (for _array_element _outactors
        (`GameplayStatics.ApplyDamage` _array_element 2.5)
        (`GameplayStatics.PlaySoundAtLocation` null _returnvalue (struct) 1.0 1.0 0.0 null null null)
        (`GameplayStatics.SpawnEmitterAtLocation` "/Game/InfinityBladeEffects/Effects/FX_Monsters/FX_Monster_Ausar/P_AU_Taunt_sparks.P_AU_Taunt_sparks" _returnvalue (`SceneComponent.K2_GetComponentRotation` _enemyposarrow)))
      (set `self.AttackIndex` 2)
      (goto _label_3 :!via `Reset`))))

(event `StopMinionCombo`
  (set `self.isAttacking` false)
  (set `self.AttackIndex` 0))

(event `MinionAttack3`
  (bind _enemyposarrow (`self.EnemyPosArrow`))
  (bind _returnvalue (`SceneComponent.K2_GetComponentLocation` _enemyposarrow))
  (`/Engine/EditorBlueprintResources/StandardMacros.DoOnce` false :!label _label_4
    (:`Completed`
      (`KismetSystemLibrary.Delay` 0.1)
      (`self.PlayAnimMontage` "/Game/maps/Enemies/PrimeHelix/Animations/attackC.attackC")
      (bind _outactors (`KismetSystemLibrary.SphereOverlapActors` (`SceneComponent.K2_GetComponentLocation` (`self.EnemyPosArrow`)) 50.0 (`|MakeArray` "ObjectTypeQuery3" :!type "EObjectTypeQuery Enum") "/Game/maps/PlayerAssets/MyAuroraCharacter_BP.MyAuroraCharacter_BP_C" (`|MakeArray` self :!type "Actor Object Reference")))
      (for _array_element _outactors
        (`GameplayStatics.ApplyDamage` _array_element 2.5)
        (`GameplayStatics.PlaySoundAtLocation` null _returnvalue (struct) 1.0 1.0 0.0 null null null)
        (`GameplayStatics.SpawnEmitterAtLocation` "/Game/InfinityBladeEffects/Effects/FX_Monsters/FX_Monster_Ausar/P_AU_Taunt_sparks.P_AU_Taunt_sparks" _returnvalue (`SceneComponent.K2_GetComponentRotation` _enemyposarrow)))
      (set `self.AttackIndex` 3)
      (goto _label_4 :!via `Reset`))))

(event `MinionAttack4`
  (bind _enemyposarrow (`self.EnemyPosArrow`))
  (bind _returnvalue (`SceneComponent.K2_GetComponentLocation` _enemyposarrow))
  (`/Engine/EditorBlueprintResources/StandardMacros.DoOnce` false :!label _label_5
    (:`Completed`
      (`KismetSystemLibrary.Delay` 0.1)
      (`self.PlayAnimMontage` "/Game/maps/Enemies/PrimeHelix/Animations/attackD.attackD")
      (bind _outactors (`KismetSystemLibrary.SphereOverlapActors` (`SceneComponent.K2_GetComponentLocation` (`self.EnemyPosArrow`)) 50.0 (`|MakeArray` "ObjectTypeQuery3" :!type "EObjectTypeQuery Enum") "/Game/maps/PlayerAssets/MyAuroraCharacter_BP.MyAuroraCharacter_BP_C" (`|MakeArray` self :!type "Actor Object Reference")))
      (for _array_element _outactors
        (`GameplayStatics.ApplyDamage` _array_element 2.5)
        (`GameplayStatics.PlaySoundAtLocation` "/Game/HumanVocalizations/HumanFemaleA/Wavs/voice_female_a_hurt_pain_10.voice_female_a_hurt_pain_10" _returnvalue (struct) 1.0 1.0 0.0 null null null)
        (`GameplayStatics.SpawnEmitterAtLocation` "/Game/InfinityBladeEffects/Effects/FX_Monsters/FX_Monster_Ausar/P_AU_Taunt_sparks.P_AU_Taunt_sparks" _returnvalue (`SceneComponent.K2_GetComponentRotation` _enemyposarrow)))
      (set `self.AttackIndex` 0)
      (goto _label_5 :!via `Reset`))))

(fn `  Attack`
  (returns (AnimationDuration :type "Float (double-precision)"))
  (`self.MinionComboAttackBTcall`)
  (return 0.4))

(fn `UserConstructionScript`)