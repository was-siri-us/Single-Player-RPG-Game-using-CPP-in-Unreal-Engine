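; BPC_AuroraStats is an actor component that stores and manages health for the Aurora player character.
; On BeginPlay it casts its owner to MyAuroraCharacter_BP and caches that reference.
; DecreaseHealth clamps health at zero and returns true when it is depleted, while IncreaseHealth caps healing at the maximum.
; SetMaxHealth sets a new maximum and refills current health to it.
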(event `self.ReceiveBeginPlay`
  (bind _asmy_aurora_character_bp (cast `/Game/maps/PlayerAssets/MyAuroraCharacter_BP` (`self.GetOwner`)))
  (set `self.As My Aurora Character BP` _asmy_aurora_character_bp))

(fn `DecreaseHealth`
  (params (Damage :type "Float (double-precision)"))
  (returns (isDead :type Boolean))
  (if (<= (- (`self.CurrentHealth`) Damage) 0.0)
    (set `self.CurrentHealth` 0.0)
    (return true)
    (else
      (set `self.CurrentHealth` (- (`self.CurrentHealth`) Damage))
      (return false))))

(fn `IncreaseHealth`
  (params (HealthPack :type "Float (double-precision)"))
  (bind _returnvalue (+ (`self.CurrentHealth`) HealthPack))
  (if (>= _returnvalue (`self.MaxHealth`))
    (set `self.CurrentHealth` (`self.MaxHealth`))
    (else
      (set `self.CurrentHealth` _returnvalue))))

(fn `SetMaxHealth`
  (params (MaxHealth :type "Float (double-precision)"))
  (bind _output_get (set `self.MaxHealth` MaxHealth))
  (set `self.CurrentHealth` _output_get))